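; Footstep anim notify that plays a surface-specific sound when triggered in an animation.
; It line traces on Visibility from the attach socket to 50 units above it, as subtracting a negative Z offset points the trace upward.
; On a hit, the physical surface type selects a concrete, metal, stone, grass or wood sound, with concrete as default.
; The sound spawns attached to the mesh socket with configurable volume and pitch multipliers.
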(fn `Received_Notify`
  (params (MeshComp :type "SkeletalMeshComponent Object Reference") (Animation :type "AnimSequenceBase Object Reference") (EventReference :type "AnimNotifyEventReference Structure (by ref)"))
  (returns (ReturnValue :type Boolean))
  (locals (FootstepLocation :type "Vector Structure"))
  (bind _output_get (set `local.FootstepLocation` (`SceneComponent.GetSocketLocation` MeshComp (`self.AttachPointName`))))
  (bind (_outhit _returnvalue) (`KismetSystemLibrary.LineTraceSingle` _output_get (- _output_get (0.0 0.0 -50.0)) "TraceTypeQuery1"))
  (if _returnvalue
    (`GameplayStatics.SpawnSoundAttached` (select `EPhysicalSurface` (`GameplayStatics.GetSurfaceType` _outhit) :`SurfaceType_Default` "/Game/Sound/Footsteps/Concrete/SC_SFX_FS_Concrete.SC_SFX_FS_Concrete" :`SurfaceType1` "/Game/Sound/Footsteps/Concrete/SC_SFX_FS_Concrete.SC_SFX_FS_Concrete" :`SurfaceType2` "/Game/Sound/Footsteps/Metal/SC_SFX_FS_Metal.SC_SFX_FS_Metal" :`SurfaceType3` "/Game/Sound/Footsteps/Stone/SC_SFX_FS_Stone.SC_SFX_FS_Stone" :`SurfaceType4` "/Game/Sound/Footsteps/Grass/SC_SFX_FS_Grass.SC_SFX_FS_Grass" :`SurfaceType5` "/Game/Sound/Footsteps/Wood/SC_SFX_FS_Wood.SC_SFX_FS_Wood" :!type "SoundBase Object Reference") (`local.MeshComp`) (`self.AttachPointName`) (0.0 0.0 0.0) (struct) "KeepRelativeOffset" false (`self.VolumeMultiplier`) (`self.PitchMultiplier`) 0.0 null null)
    (return false)))