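; BP_AMB2 is an ambient sound switcher that swaps between indoor and outdoor ambience as the FirstPersonCharacter moves between two trigger boxes.
; Overlapping BoxIn starts AmbIn and fades out AmbOut, while overlapping BoxOut does the reverse.
; An Isinside flag makes each box act only on a change of state, with the incoming sound starting instantly and the outgoing one fading briefly.
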(event `self.BoxIn.OnComponentBeginOverlap`
  (params (OverlappedComponent :type "PrimitiveComponent Object Reference") (OtherActor :type "Actor Object Reference") (OtherComp :type "PrimitiveComponent Object Reference") (OtherBodyIndex :type Integer) (bFromSweep :type Boolean) (SweepResult :type "HitResult Structure (by ref)"))
  (cast `/Game/Blueprints/Player/FirstPersonCharacter` OtherActor)
  (if (not (`self.Isinside`))
    (`AudioComponent.FadeIn` (`AmbientSound.AudioComponent` (`self.AmbIn`)) 0.0 1.0 0.0 "Linear")
    (`AudioComponent.FadeOut` (`AmbientSound.AudioComponent` (`self.AmbOut`)) 0.5 0.0 "Linear")
    (set `self.Isinside` true)))

(event `self.BoxOut.OnComponentBeginOverlap`
  (params (OverlappedComponent :type "PrimitiveComponent Object Reference") (OtherActor :type "Actor Object Reference") (OtherComp :type "PrimitiveComponent Object Reference") (OtherBodyIndex :type Integer) (bFromSweep :type Boolean) (SweepResult :type "HitResult Structure (by ref)"))
  (cast `/Game/Blueprints/Player/FirstPersonCharacter` OtherActor)
  (if (`self.Isinside`)
    (`AudioComponent.FadeIn` (`AmbientSound.AudioComponent` (`self.AmbOut`)) 0.0 1.0 0.0 "Linear")
    (`AudioComponent.FadeOut` (`AmbientSound.AudioComponent` (`self.AmbIn`)) 0.5 0.0 "Linear")
    (set `self.Isinside` false)))

(fn `UserConstructionScript`)